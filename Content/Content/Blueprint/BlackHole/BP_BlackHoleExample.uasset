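; Example black hole actor that turns toward the local player and reacts to actors it is about to destroy.
; Each tick, if player character 0 is locally controlled, it applies the look-at yaw and roll toward that character with pitch zeroed.
; OnDestroyActor is a hook for pre-destruction logic, here printing a game-over message for the player or the actor's name otherwise.
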(event `self.ReceiveTick`
  (params (DeltaSeconds :type "Float (single-precision)"))
  (bind _returnvalue (`GameplayStatics.GetPlayerCharacter` 0))
  ;[1 1 1] Set Hole Rotation
  (`/Engine/EditorBlueprintResources/StandardMacros.IsValid` _returnvalue
    (:`Is Valid`
      (if (`Pawn.IsLocallyControlled` _returnvalue)
        (`self.K2_SetActorRotation` (`KismetMathLibrary.MakeRotator` (.roll (`KismetMathLibrary.FindLookAtRotation` (`self.K2_GetActorLocation`) (`self.K2_GetActorLocation` _returnvalue))) 0.0 (.yaw (`KismetMathLibrary.FindLookAtRotation` (`self.K2_GetActorLocation`) (`self.K2_GetActorLocation` _returnvalue)))))))))

(event `self.OnDestroyActor`
  (params (Actor :type "Actor Object Reference"))
  ;[1 1 1] Activates events in the actors before it is destroyed. Example: Activate the character death event before the character is destroyed
  (`KismetSystemLibrary.PrintString` (select `bool` (== Actor (`GameplayStatics.GetPlayerCharacter` 0)) :`false` (`KismetSystemLibrary.GetDisplayName` Actor) :`true` "Game Over :(")))

(fn `UserConstructionScript`)